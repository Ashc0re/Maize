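; BP_Pickup is an interactable pickup that adds an item to the interacting player's inventory.
; Its Interacted override appends an entry built from Item and Amount to the Inventory, then calls the parent implementation.
; If the Inventory already contains an entry matching Item with zeroed remaining fields, it only prints a placeholder "Hello", with no stacking.
; The event graph holds only disabled default events.
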(event EventBeginPlay
  (|CallParentFunction) ; This node is disabled and will not be called.\nDrag off pins to build functionality.
)

(event Collision|EventActorBeginOverlap
  (params (OtherActor :type Actor%20Object%20Reference))
  (|CallParentFunction OtherActor) ; This node is disabled and will not be called.\nDrag off pins to build functionality.
)

(event EventTick
  (params (DeltaSeconds :type Float%20%28single-precision%29))
  (|CallParentFunction DeltaSeconds) ; This node is disabled and will not be called.\nDrag off pins to build functionality.
)

(fn ConstructionScript
  (|CallParentFunction))

(fn Interacted
  (params (Player :type BP%20Player%20Object%20Reference))
  (bind _inventory (Variables|/Game/Blueprint/Player/BP_Player.BP_Player_C|GetInventory Player))
  (if (Utilities|Array|ContainsItem _inventory (Utilities|Struct|MakeStruct_Item (Variables|Default|GetItem) 0 0))
    (Development|PrintString "Hello")
    (else
      (Utilities|Array|Add _inventory (Utilities|Struct|MakeStruct_Item (Variables|Default|GetItem) (Variables|Default|GetAmount) 0))
      (|CallParentFunction 0))))
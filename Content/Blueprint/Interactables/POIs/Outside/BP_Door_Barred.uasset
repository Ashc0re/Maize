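; BP_Door_Barred is an outdoor interactable door that stays locked until the board barring it is removed.
; It overrides InteractedWithComponent: interacting with the board sets Unlocked, rebuilds the interactable component states and destroys the board.
; Interacting with the door destroys it and calls the parent handler when unlocked, otherwise it only prints a locked message.
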(fn ConstructionScript
  (|CallParentFunction))

(fn InteractedwithComponent
  (params (Component :type Static%20Mesh%20Component%20Object%20Reference) (Player_ :type BP%20Player%20Base%20Object%20Reference))
  (LocalVariables|Set_Component Component)
  (Utilities|FlowControl|Sequence
    (:then_0
      (if (== (LocalVariables|Get_Component) (Variables|Default|GetSM_Door))
        (if (Variables|Default|GetUnlocked)
          (Components|DestroyComponent (Variables|Default|GetSM_Door))
          (|CallParentFunction (LocalVariables|Get_Component) Player_)
          (else
            (Development|PrintString "Locked!")))))
    (:then_1
      (if (== (LocalVariables|Get_Component) (Variables|Default|GetSM_Board))
        (Variables|Default|SetUnlocked true)
        (Variables|Default|SetInteractComponents (Utilities|Array|MakeArray (Utilities|Struct|MakeStruct_InteractableComponentState "/Game/3D/Door_Barred/SM_Door.SM_Door" 1.0 true) (Utilities|Struct|MakeStruct_InteractableComponentState "/Game/3D/Door_Barred/SM_Board.SM_Board" 0.5 false)))
        (Components|DestroyComponent (Variables|Default|GetSM_Board))))))
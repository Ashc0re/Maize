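; Outdoor gate button interactable that runs a staged fuse puzzle, currently ending in a "Gate Open!" debug print.
; The first press blows the fuse and unlocks the lid, whose removal consumes required items and exposes the fuse slot.
; The slot takes two interactions, removal then item-consuming insertion, before the button succeeds.
; Stages are gated by booleans and by helpers that rewrite the InteractComponents array entries by index.
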(fn ConstructionScript
  (|CallParentFunction))

(fn InteractedwithComponent
  (params (Component :type Static%20Mesh%20Component%20Object%20Reference) (Player_ :type BP%20Player%20Base%20Object%20Reference))
  (LocalVariables|Set_Component Component)
  (LocalVariables|Set_Player Player_)
  (Utilities|FlowControl|Sequence
    (:then_0
      ;[0.15 0.15 0.15 0.5] Button
      (if (== (LocalVariables|Get_Component) (Variables|Default|GetButton))
        (if (Variables|Default|GetFuseBlown)
          (if (Variables|Default|GetFuseInserted)
            (Development|PrintString "Gate Open!")
            (|CallParentFunction (LocalVariables|Get_Component) 0 :!label _label))
          (else
            (Variables|Default|SetFuseBlown true)
            (Audio|PlaySoundatLocation "/Engine/VREditor/Sounds/VR_teleport.VR_teleport" (Transformation|GetWorldLocation (Variables|Default|GetDefaultSceneRoot)) "0, 0, 0" 1.0 1.0 0.0 0 0 0 0)
            (CallFunction|SetComponentInteractable 1 true)
            (goto _label)))))
    (:then_1
      ;[0.15 0.15 0.15 0.5] Lid
      (if (and (Variables|Default|GetFuseBlown) (== (LocalVariables|Get_Component) (Variables|Default|GetLid)))
        (bind _itemsrequired (CallFunction|GetComponentInteractItems (LocalVariables|Get_Component)))
        (for _array_element _itemsrequired
          (Default|InventoryRemoveItem (LocalVariables|Get_Player) _array_element 1))
        (Components|DestroyComponent (Variables|Default|GetLid))
        (CallFunction|SetComponentInteractable 2 true)
        (goto _label)))
    (:then_2
      ;[0.15 0.15 0.15 0.5] Fuse
      (if (and (Variables|Default|GetFuseBlown) (== (LocalVariables|Get_Component) (Variables|Default|GetFuseSlot)))
        (if (Variables|Default|GetFuseRemoved)
          (bind (_componentfound _itemsrequired_2) (CallFunction|GetComponentInteractItems (LocalVariables|Get_Component)))
          (if _componentfound
            (for _array_element_2 _itemsrequired_2
              (Default|InventoryRemoveItem (LocalVariables|Get_Player) _array_element_2 1))
            (Variables|Default|SetFuseInserted true)
            (Rendering|Material|SetMaterial (Variables|Default|GetSM_Fuse) 0 "/Game/3D/Fuse/Materials/M_Fuse.M_Fuse")
            (Rendering|SetVisibility (Variables|Default|GetSM_Fuse) true false)
            (goto _label))
          (else
            (Variables|Default|SetFuseRemoved true)
            (Rendering|SetVisibility (Variables|Default|GetSM_Fuse) true false)))))))

(fn SetComponentInteractTime
  (params (Index :type Integer) (New%20Interact%20Time :type Float%20%28double-precision%29))
  (bind _interactcomponents (Variables|Default|GetInteractComponents))
  (bind _output (Utilities|Array|Get(acopy) _interactcomponents Index))
  (bind (_staticmesh _interacttime _isinteractable _itemsrequired) (Utilities|Struct|BreakStruct_InteractableComponentState _output))
  (Utilities|Array|SetArrayElem (Variables|Default|GetInteractComponents) Index (Utilities|Struct|MakeStruct_InteractableComponentState _staticmesh New%20Interact%20Time _isinteractable _itemsrequired)))

(fn SetComponentInteractable
  (params (Index :type Integer) (Interactable :type Boolean))
  (bind _interactcomponents (Variables|Default|GetInteractComponents))
  (bind _output (Utilities|Array|Get(acopy) _interactcomponents Index))
  (bind (_staticmesh _interacttime _isinteractable _itemsrequired) (Utilities|Struct|BreakStruct_InteractableComponentState _output))
  (Utilities|Array|SetArrayElem (Variables|Default|GetInteractComponents) Index (Utilities|Struct|MakeStruct_InteractableComponentState _staticmesh _interacttime Interactable _itemsrequired)))
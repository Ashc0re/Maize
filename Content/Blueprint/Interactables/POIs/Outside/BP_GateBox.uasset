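; Outdoor gate control box interactable that runs a blown-fuse repair puzzle.
; The first completed button press blows the fuse, damages the player and makes the lid interactable.
; Removing the lid consumes required items and unlocks the fuse slot, where the fuse is removed, then replaced from inventory.
; InteractComponents entries gate each step; pressing the button after repair only prints a gate-open message.
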(fn ConstructionScript
  (|CallParentFunction))

(fn InteractionStarted
  (params (Component :type Static%20Mesh%20Component%20Object%20Reference) (Player_ :type BP%20Player%20Base%20Object%20Reference))
  (Utilities|FlowControl|Sequence
    (:then_0
      ;[0.15 0.15 0.15 0.5] Button
      (if (== Component (Variables|Default|GetButton))
        (CallFunction|PlayInteractSound "NewEnumerator0" "/Engine/VREditor/Sounds/UI/Gizmo_Handle_Clicked.Gizmo_Handle_Clicked")))))

(fn SetComponentInteractTime
  (params (Index :type Integer) (New%20Interact%20Time :type Float%20%28double-precision%29))
  (bind _interactcomponents (Variables|Default|GetInteractComponents))
  (bind _output (Utilities|Array|Get(acopy) _interactcomponents Index))
  (bind (_staticmesh _interacttime _isinteractable _itemsrequired) (Utilities|Struct|BreakStruct_InteractableComponentState _output))
  (Utilities|Array|SetArrayElem (Variables|Default|GetInteractComponents) Index (Utilities|Struct|MakeStruct_InteractableComponentState _staticmesh New%20Interact%20Time _isinteractable _itemsrequired 0 0)))

(fn SetComponentInteractable
  (params (Index :type Integer) (Interactable :type Boolean))
  (bind _interactcomponents (Variables|Default|GetInteractComponents))
  (bind _output (Utilities|Array|Get(acopy) _interactcomponents Index))
  (bind (_staticmesh _interacttime _isinteractable _itemsrequired) (Utilities|Struct|BreakStruct_InteractableComponentState _output))
  (Utilities|Array|SetArrayElem (Variables|Default|GetInteractComponents) Index (Utilities|Struct|MakeStruct_InteractableComponentState _staticmesh _interacttime Interactable _itemsrequired 0 0)))

(fn InteractionComplete
  (params (Player :type BP%20Player%20Base%20Object%20Reference) (Component :type Static%20Mesh%20Component%20Object%20Reference))
  (Utilities|FlowControl|Sequence
    (:then_0
      ;[0.15 0.15 0.15 0.5] Button
      (if (== Component (Variables|Default|GetButton))
        (if (Variables|Default|GetFuseBlown)
          (if (Variables|Default|GetFuseInserted)
            (Development|PrintString "Gate Open!"))
          (CallFunction|PlayInteractSound "NewEnumerator0" "/Engine/VREditor/Sounds/UI/Gizmo_Handle_Clicked.Gizmo_Handle_Clicked")
          (else
            (Variables|Default|SetFuseBlown true)
            (CallFunction|SetComponentInteractable 1 true)
            (CallFunction|PlayInteractSound "NewEnumerator0" "/Engine/VREditor/Sounds/VR_teleport.VR_teleport")
            (Default|TakeDamage Player 40)))))
    (:then_1
      ;[0.15 0.15 0.15 0.5] Lid
      (if (and (Variables|Default|GetFuseBlown) (== Component (Variables|Default|GetLid)))
        (bind _itemsrequired (CallFunction|GetComponentInteractItems Component))
        (for _array_element _itemsrequired
          (Default|InventoryRemoveItem Player _array_element 1))
        (Components|DestroyComponent (Variables|Default|GetLid))
        (CallFunction|SetComponentInteractable 2 true)))
    (:then_2
      ;[0.15 0.15 0.15 0.5] Fuse
      (if (and (Variables|Default|GetFuseBlown) (== Component (Variables|Default|GetFuseSlot)))
        (if (Variables|Default|GetFuseRemoved)
          (bind (_componentfound _itemsrequired_2) (CallFunction|GetComponentInteractItems Component))
          (if _componentfound
            (for _array_element_2 _itemsrequired_2
              (Default|InventoryRemoveItem Player _array_element_2 1))
            (Variables|Default|SetFuseInserted true)
            (Rendering|Material|SetMaterial (Variables|Default|GetSM_Fuse) 0 "/Game/3D/Fuse/Materials/M_Fuse.M_Fuse")
            (Rendering|SetVisibility (Variables|Default|GetSM_Fuse) true false))
          (else
            (Variables|Default|SetFuseRemoved true)
            (Rendering|SetVisibility (Variables|Default|GetSM_Fuse) false false)))))))
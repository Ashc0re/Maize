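; BP_Interactable is an interactable actor with empty hooks for a player interacting with the actor or one of its components.
; An InteractComponents array supplies each component's interactable flag, interact time and required items through lookup functions.
; Lookups match on static mesh asset rather than component reference, so components sharing a mesh resolve to the first matching entry.
; The required-items lookup also prints the component's name.
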(fn ConstructionScript)

(fn InteractedwithActor
  (params (Player :type BP%20Player%20Base%20Object%20Reference)))

(fn InteractedwithComponent
  (params (Component :type Static%20Mesh%20Component%20Object%20Reference) (Player_ :type BP%20Player%20Base%20Object%20Reference)))

(fn GetComponentInteractTime
  (params (Component :type Static%20Mesh%20Component%20Object%20Reference))
  (for _array_element (Variables|Default|GetInteractComponents)
    (if (== (.StaticMesh (Utilities|Struct|BreakStruct_InteractableComponentState _array_element)) (Variables|/Script/Engine.StaticMeshComponent|GetStaticMesh Component))
      (return true (.InteractTime (Utilities|Struct|BreakStruct_InteractableComponentState _array_element)))))
  (return false 0.0))

(fn GetComponentInteractItems
  (params (Component :type Static%20Mesh%20Component%20Object%20Reference))
  (Development|PrintString (Utilities|GetDisplayName Component))
  (for _array_element (Variables|Default|GetInteractComponents)
    (if (== (.StaticMesh (Utilities|Struct|BreakStruct_InteractableComponentState _array_element)) (Variables|/Script/Engine.StaticMeshComponent|GetStaticMesh Component))
      (return true (.ItemsRequired (Utilities|Struct|BreakStruct_InteractableComponentState _array_element)))))
  (return false 0))

(fn IsComponentInteractable
  (params (Component :type Static%20Mesh%20Component%20Object%20Reference))
  (for _array_element (Variables|Default|GetInteractComponents)
    (if (== (.StaticMesh (Utilities|Struct|BreakStruct_InteractableComponentState _array_element)) (Variables|/Script/Engine.StaticMeshComponent|GetStaticMesh Component))
      (return (.Interactable (Utilities|Struct|BreakStruct_InteractableComponentState _array_element)))))
  (return false))
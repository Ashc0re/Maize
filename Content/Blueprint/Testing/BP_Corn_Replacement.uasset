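; BP_Corn_Replacement is a test actor that stands in for a single corn plant instance in a corn field.
; Initialization stores the instance index, the field reference and the transform.
; Show and hide events play a scale timeline forward or in reverse, resizing both collider and mesh.
; Logic to restore the field instance at unit scale is disconnected, and the timeline's finish branch does nothing.
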(event Custom|Event_ShowPlant
  (bind (_direction _scale) (Timeline|TL_Scale PlayFromStart)
    (:Update
      (Transformation|SetRelativeScale3D (Variables|Default|GetCollider) (Math|Conversions|ToVector(Float) _scale))
      (Transformation|SetRelativeScale3D (Variables|Default|GetMesh) (Math|Conversions|ToVector(Float) _scale)))
    (:Finished
      (if (Utilities|Enum|Equal(Enum) _direction "Forward")
        _))))

(event Custom|Event_HidePlant
  (bind (_direction _scale) (Timeline|TL_Scale ReverseFromEnd)
    (:Update
      (Transformation|SetRelativeScale3D (Variables|Default|GetCollider) (Math|Conversions|ToVector(Float) _scale))
      (Transformation|SetRelativeScale3D (Variables|Default|GetMesh) (Math|Conversions|ToVector(Float) _scale)))
    (:Finished
      (if (Utilities|Enum|Equal(Enum) _direction "Forward")
        _))))

(event Custom|Event_Initialize
  (params (Index :type Integer) (CornField :type Instanced%20Static%20Mesh%20Component%20Object%20Reference) (Transform :type Transform))
  (Variables|Default|SetIndex Index)
  (Variables|Default|SetCornField CornField)
  (Variables|Default|SetTransform Transform))

(fn ConstructionScript)
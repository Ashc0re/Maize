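; Base handler that spawns, logs and despawns scarecrow enemies for an area, using its BP_Scarecrow_Spawn points split into forced and optional lists.
; Forced points roll their own weighted enemy map, falling back to a stationary scarecrow.
; Optional points are shuffled, then filled round-robin by enemy type under percentage-based caps.
; Despawning destroys only tracked enemies, which exclude forced spawns other than fallbacks.
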(fn ConstructionScript)

(fn PopulateScarecrowSpawns
  (params (Area :type Enum_Areas%20Enum :default "NewEnumerator0"))
  (LocalVariables|Set_Area Area)
  (bind _outactors (Actor|GetAllActorsOfClass "/Game/Blueprint/Scarecrows/BP_Scarecrow_Spawn.BP_Scarecrow_Spawn_C"))
  (for _array_element _outactors
    (LocalVariables|Set_Spawnpoint _array_element)
    (if (Utilities|Enum|Equal(Enum) (Variables|/Game/Blueprint/Scarecrows/BP_Scarecrow_Spawn.BP_Scarecrow_Spawn_C|GetArea _array_element) (LocalVariables|Get_Area))
      (if (Variables|/Game/Blueprint/Scarecrows/BP_Scarecrow_Spawn.BP_Scarecrow_Spawn_C|GetForceSpawn (LocalVariables|Get_Spawnpoint))
        (Utilities|Array|Add (Variables|SpawnLogic|GetSpawns_Forced) (LocalVariables|Get_Spawnpoint))
        (else
          (Utilities|Array|Add (Variables|SpawnLogic|GetSpawns_Optional) (LocalVariables|Get_Spawnpoint)))))))

(fn InitiateSpawns
  (CallFunction|LogInitiateSpawns)
  (Utilities|FlowControl|Sequence
    (:then_0
      ;[0.15 0.15 0.15 0.5] Initiate Forced Spawns
      (Utilities|Error:NoSpawnFound (Variables|SpawnLogic|GetSpawns_Forced)
        (:SpawnsFound
          ;;[0.15 0.15 0.15 0.5] Spawn Scarecrows at each Forced Spawn
          (for _array_element (Variables|SpawnLogic|GetSpawns_Forced)
            (Utilities|Error:InvalidSpawn _array_element
              (:IsValid
                (bind (__enemyspawned __spawnlocation) (CallFunction|SpawnForcedScarecrow _array_element))
                (CallFunction|LogScarecrowSpawn __enemyspawned __spawnlocation)))))))
    (:then_1
      ;[0.15 0.15 0.15 0.5] Initiate Optional Spawns
      (Utilities|Error:NoSpawnFound (Variables|SpawnLogic|GetSpawns_Optional)
        (:SpawnsFound
          ;;[0.15 0.15 0.15 0.5] Randomize Spawn Locations
          (Utilities|Array|Shuffle (Variables|SpawnLogic|GetSpawns_Optional))
          ;;[0.15 0.15 0.15 0.5] Calculate number of maximum possible spawns for each enemy type seperatly
          (bind _valuepin (Utilities|Map|ForEachLoop(Map) (Variables|Parameters|GetEnemiesToSpawn))
            (:then
              (CallFunction|CalculateNumberOfPossibleSpawns _valuepin))
            (:CompletedPin
              ;;[0.15 0.15 0.15 0.5] Populate an Array used to check how many enemies of each type have already been spawned. Starts with 0 Enemies per type
              (for _array_element_2 (Variables|SpawnLogic|GetNumberOfPossibleSpawns)
                (Utilities|Array|Add (Variables|SpawnLogic|GetEnemiesSpawned) 0))
              (for _array_element_3 (Variables|SpawnLogic|GetSpawns_Optional)
                ;;[0.15 0.15 0.15 0.5] Spawn an pseudo-random amount of enemies based on their spawn chance
                (bind (_enemytospawn _enemyindex) (CallFunction|GetEnemytoSpawn (LocalVariables|Get_LastEnemySpawned)))
                ;;;[0.15 0.15 0.15 0.5] Making sure each enemy type has a fair chance of getting spawned resulting in pseudo-random spawnrates
                (bind _result (Math|Integer|IncrementInt _enemyindex)
                  (:%20%20
                    (bind _output_get (LocalVariables|Set_LastEnemySpawned _result))
                    (if (>= _output_get (Utilities|Map|Length (Variables|Parameters|GetEnemiesToSpawn)))
                      (LocalVariables|Set_LastEnemySpawned 0))
                    (bind (__enemyspawned_2 __spawnlocation_2) (CallFunction|SpawnRandomScarecrow _array_element_3 _enemytospawn))
                    (CallFunction|LogScarecrowSpawn __enemyspawned_2 __spawnlocation_2)))))))))))

(fn DespawnEnemies
  ;[0.15 0.15 0.15 0.5] Destroy all enemy actors
  (for _array_element (Variables|AreaHandling|GetEnemiesPresent)
    (Actor|DestroyActor _array_element)
    ;[0.15 0.15 0.15 0.5] Clear spawn counter
    (Utilities|Array|Clear (Variables|SpawnLogic|GetEnemiesSpawned))))

(fn SpawnRandomScarecrow
  (params (Spawn :type BP%20Scarecrow%20Spawn%20Object%20Reference) (EnemyToSpawn :type BP%20Scarecrow%20Class%20Reference))
  (LocalVariables|Set_Spawn Spawn)
  (bind _returnvalue (Game|SpawnActorfromClass EnemyToSpawn (Math|Transform|MakeTransform (Transformation|GetActorLocation (LocalVariables|Get_Spawn)) (Transformation|GetActorRotation (LocalVariables|Get_Spawn))) "Undefined" "MultiplyWithRoot" 0 0))
  ;[0.15 0.15 0.15 0.5] Update array of all enemies currently present in area
  (Utilities|Array|Add (Variables|AreaHandling|GetEnemiesPresent) _returnvalue)
  (return _returnvalue (LocalVariables|Get_Spawn)))

(fn SpawnForcedScarecrow
  (params (Spawn :type BP%20Scarecrow%20Spawn%20Object%20Reference))
  (bind _output_get (LocalVariables|Set_Spawn Spawn))
  (if (Variables|/Game/Blueprint/Scarecrows/BP_Scarecrow_Spawn.BP_Scarecrow_Spawn_C|GetForceSpawn _output_get)
    ;[0.15 0.15 0.15 0.5] Get Random Enemy To Spawn
    (bind (_keypin _valuepin) (Utilities|Map|ForEachLoop(Map) (Variables|/Game/Blueprint/Scarecrows/BP_Scarecrow_Spawn.BP_Scarecrow_Spawn_C|GetEnemiesToSpawn (LocalVariables|Get_Spawn)))
      (:then
        (bind _output_get_2 (LocalVariables|SetAccumulatedWeight (+ _valuepin (LocalVariables|GetAccumulatedWeight))))
        (if (<= (Math|Random|RandomFloat) _output_get_2)
          (LocalVariables|SetSpawned true)
          (bind _returnvalue (Game|SpawnActorfromClass _keypin (Math|Transform|MakeTransform (Transformation|GetActorLocation (LocalVariables|Get_Spawn)) (Transformation|GetActorRotation (LocalVariables|Get_Spawn))) "AdjustIfPossibleButAlwaysSpawn" "MultiplyWithRoot" 0 0))
          (return _returnvalue (LocalVariables|Get_Spawn))))
      (:CompletedPin
        ;[0.15 0.15 0.15 0.5] Spawn a fallback enemy if no enemy has been spawned
        (if (not (LocalVariables|GetSpawned))
          (bind _returnvalue_2 (Game|SpawnActorfromClass "/Game/Blueprint/Scarecrows/BP_Scarecrow_Stationary.BP_Scarecrow_Stationary_C" (Math|Transform|MakeTransform (Transformation|GetActorLocation (LocalVariables|Get_Spawn)) (Transformation|GetActorRotation (LocalVariables|Get_Spawn))) "AdjustIfPossibleButAlwaysSpawn" "MultiplyWithRoot" 0 0))
          (Utilities|Array|Add (Variables|AreaHandling|GetEnemiesPresent) _returnvalue_2)
          (return _returnvalue_2 (LocalVariables|Get_Spawn)))))))

(fn CalculateNumberOfPossibleSpawns
  (params (Percentage :type Float%20%28double-precision%29))
  (Utilities|Array|Add (Variables|SpawnLogic|GetNumberOfPossibleSpawns) (Math|Float|Ceil (* Percentage (Utilities|Array|Length (Variables|SpawnLogic|GetSpawns_Optional)))))
  (return))

(fn GetEnemytoSpawn
  (params (IndexOfLastEnemy :type Integer))
  (LocalVariables|Set_Index IndexOfLastEnemy)
  ;[0.15 0.15 0.15 0.5] Logic to pick an enemy to spawn
  ;;[0.15 0.15 0.15 0.5] Check each enemy once
  (Utilities|Map|ForEachLoop(Map) (Variables|Parameters|GetEnemiesToSpawn)
    (:then
      ;;[0.15 0.15 0.15 0.5] Check if enemy is allowed to spawn
      (LocalVariables|Set_EnemiesOfTypeSpawned (Utilities|Array|Get(acopy) (Variables|SpawnLogic|GetEnemiesSpawned) (LocalVariables|Get_Index)))
      (if (<= (Utilities|Array|Get(acopy) (Variables|SpawnLogic|GetEnemiesSpawned) (LocalVariables|Get_Index)) (Utilities|Array|Get(acopy) (Variables|SpawnLogic|GetNumberOfPossibleSpawns) (LocalVariables|Get_Index)))
        ;;[0.15 0.15 0.15 0.5] Update the amount of enemies of the current type spawend
        (bind _result (Math|Integer|IncrementInt (LocalVariables|Get_EnemiesOfTypeSpawned))
          (:%20%20
            (Utilities|Array|SetArrayElem (Variables|SpawnLogic|GetEnemiesSpawned) (LocalVariables|Get_Index) _result)
            ;[0.15 0.15 0.15 0.5] Return enemy to spawn and its index
            (return (.Key (Utilities|Map|GetKeyValueByIndex (Variables|Parameters|GetEnemiesToSpawn) (LocalVariables|Get_Index))) (LocalVariables|Get_Index))))
        (else
          ;;[0.15 0.15 0.15 0.5] Increase Index by one to check next enemy type during next loop
          (Math|Integer|IncrementInt (LocalVariables|Get_Index)))))))

(fn LogScarecrowSpawn
  (params (Enemy :type BP%20Scarecrow%20Object%20Reference) (Spawn :type BP%20Scarecrow%20Spawn%20Object%20Reference))
  (LocalVariables|Set_Enemy Enemy)
  (LocalVariables|Set_Spawn Spawn)
  (if (and (Utilities|IsValid Enemy) (Utilities|IsValid Spawn))
    (if (Variables|/Game/Blueprint/Scarecrows/BP_Scarecrow_Spawn.BP_Scarecrow_Spawn_C|GetForceSpawn (LocalVariables|Get_Spawn))
      (Utilities|String|LogString (Utilities|String|Append "Froced spawn of " (Utilities|String|Append (Utilities|GetClassDisplayName (Utilities|GetClass (LocalVariables|Get_Enemy))) " in area " (Utilities|String|EnumtoString (Variables|/Game/Blueprint/Scarecrows/BP_Scarecrow_Spawn.BP_Scarecrow_Spawn_C|GetArea (LocalVariables|Get_Spawn))) ", at spawn with the following descriptor: " (Variables|/Game/Blueprint/Scarecrows/BP_Scarecrow_Spawn.BP_Scarecrow_Spawn_C|GetDescriptor (LocalVariables|Get_Spawn)))))
      (else
        (Utilities|String|LogString (Utilities|String|Append "Spawned " (Utilities|String|Append (Utilities|GetClassDisplayName (Utilities|GetClass (LocalVariables|Get_Enemy))) " in area " (Utilities|String|EnumtoString (Variables|/Game/Blueprint/Scarecrows/BP_Scarecrow_Spawn.BP_Scarecrow_Spawn_C|GetArea (LocalVariables|Get_Spawn))) ", at spawn with the following descriptor: " (Variables|/Game/Blueprint/Scarecrows/BP_Scarecrow_Spawn.BP_Scarecrow_Spawn_C|GetDescriptor (LocalVariables|Get_Spawn)))))))
    (else
      (Utilities|Debugging|RaiseScriptError "Failed to log Scarecrow spawn!"))))

(fn LogInitiateSpawns
  (Utilities|String|LogString (Utilities|String|Append "Initiated spawns in the following area: " (Utilities|String|EnumtoString (Variables|Parameters|GetArea)))))
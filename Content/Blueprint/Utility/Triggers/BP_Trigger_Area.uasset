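; BP_Trigger_Area is a trigger volume that drives enemy spawning when the player walks into it.
; On overlap by BP_Player_Base, it tells the entered handler to spawn enemies and, optionally, the left handler to despawn its enemies.
; A TriggerOnce flag limits this to the first overlap; otherwise it fires on every entry.
; Both calls go through a shared helper that validates the handler before use.
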(event OnComponentBeginOverlap(Collision)
  (params (OverlappedComponent :type Primitive%20Component%20Object%20Reference) (OtherActor :type Actor%20Object%20Reference) (OtherComp :type Primitive%20Component%20Object%20Reference) (OtherBodyIndex :type Integer) (bFromSweep :type Boolean) (SweepResult :type Hit%20Result%20Structure%20%28by%20ref%29))
  ;[0.15 0.15 0.15 0.5] Check if the player has triggered this
  (Utilities|Casting|CastToBP_Player_Base OtherActor)
  (if (Variables|Default|GetTriggerOnce)
    (if (not (Variables|Default|GetTriggered))
      (Variables|Default|SetTriggered true)
      (Utilities|FlowControl|Sequence :!label _label
        (:then_0
          (CallFunction|Spawn/DespawnEnemies true (Variables|Default|GetEnteredHandler)))
        (:then_1
          (if (Variables|Default|GetDespawnEnemies)
            (CallFunction|Spawn/DespawnEnemies false (Variables|Default|GetLeftHandler))))))
    (else
      (goto _label))))

(fn ConstructionScript
  (|CallParentFunction))

(fn Spawn/DespawnEnemies
  (params (SpawnEnemies :type Boolean) (Handler :type BP%20Handler%20Base%20Object%20Reference))
  (bind _output_get (LocalVariables|Set_Handler Handler))
  (Utilities|IsValid _output_get
    (:Is%20Valid
      (if SpawnEnemies
        (Default|InitiateSpawns (LocalVariables|Get_Handler))
        (else
          (Default|DespawnEnemies (LocalVariables|Get_Handler)))))))
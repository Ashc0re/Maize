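; Trigger actor that shows a tutorial text to the player on overlap.
; On begin overlap it casts the other actor to BP_Player_Base, calls EventShowTutorialText with its Text and Duration, then marks itself triggered.
; It fires only while TriggerOnce is set and Triggered is false, so it never repeats and does nothing when TriggerOnce is off.
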(event Collision|EventActorBeginOverlap
  (params (OtherActor :type Actor%20Object%20Reference))
  (if (and (Variables|Default|GetTriggerOnce) (not (Variables|Default|GetTriggered)))
    (bind _asbp_player_base (Utilities|Casting|CastToBP_Player_Base OtherActor))
    (Default|EventShowTutorialText _asbp_player_base (Variables|Default|GetText) (Variables|Default|GetDuration))
    (Variables|Default|SetTriggered true)))

(fn ConstructionScript
  (|CallParentFunction))
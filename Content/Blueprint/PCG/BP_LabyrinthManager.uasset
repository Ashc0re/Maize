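; Labyrinth manager that generates paths through a cornfield at BeginPlay by linking BP_Knot actors attached to the Cornfield.
; It builds a BP_Quad tree over the field bounds for radius-based knot queries.
; From each House knot, it greedily steps to the in-range, unvisited knot nearest that House's target, spawning spline BP_Path actors tied to the cornfield's PCG component.
; Optional debug draws show quads and nearest knots.
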(event EventBeginPlay
  (Labyrinth|GenerateLabyrinth)
  (CallFunction|DebugDrawNearestKnottoDebugCube))

(fn ConstructionScript)

(fn PopulateKnotsArray
  (for _array_element (Actor|GetAttachedActors (Variables|Default|GetCornfield) true false)
    (bind _asbp_knot (Utilities|Casting|CastToBP_Knot _array_element))
    (Utilities|Array|Add (Variables|Default|GetKnots) _asbp_knot)))

(fn DrawPath
  (params (Start%20Knot :type Actor%20Object%20Reference) (End%20Knot :type Actor%20Object%20Reference))
  (bind _returnvalue (Game|SpawnActorfromClass "/Game/Blueprint/PCG/BP_Path.BP_Path_C" (Transformation|GetActorTransform Start%20Knot) "Undefined" "MultiplyWithRoot" (Variables|Default|GetCornfield) 0))
  (bind _output_get (LocalVariables|SetNewPath _returnvalue))
  (Spline|AddSplinePoint (Variables|/Game/Blueprint/PCG/BP_Path.BP_Path_C|GetSpline _output_get) (Transformation|GetActorLocation End%20Knot) "World" true)
  (Variables|/Game/Blueprint/PCG/BP_Path.BP_Path_C|SetCornfieldPCG (LocalVariables|GetNewPath) (Variables|/Game/Blueprint/PCG/BP_Cornfield.BP_Cornfield_C|GetPCG_Component (Variables|Default|GetCornfield)))
  (Utilities|Array|Add (Variables|Default|GetPaths) (LocalVariables|GetNewPath)))

(fn GenerateLabyrinth
  (bind _cornfield (Variables|Default|GetCornfield))
  (bind _spline_acre (Variables|/Game/Blueprint/PCG/BP_Cornfield.BP_Cornfield_C|GetSpline_Acre _cornfield))
  (bind (_origin _boxextent) (Collision|GetComponentBounds _spline_acre))
  (Knots|PopulateKnotsArray)
  (Labyrinth|ResetLabyrinth)
  (Quads|CreateRootQuad (Variables|Default|GetKnots) _origin (Math|Float|SnapToGrid(Float) (.X (Math|Vector|BreakVector _boxextent)) 1e+01) (Variables|Default|GetKnotThreshold))
  (CallFunction|BuildPathtoTarget))

(fn ResetLabyrinth
  (for _array_element (Variables|Default|GetPaths)
    (Actor|DestroyActor _array_element))
  (Utilities|Array|Clear (Variables|Default|GetPaths)))

(fn CreateRootQuad
  (params (Knots :type Array%20of%20BP%20Knot%20Object%20References) (Location :type Vector) (Length :type Float%20%28double-precision%29) (KnotThreshold :type Integer))
  (bind _returnvalue (Game|AddComponentbyClass "/Game/Blueprint/PCG/BP_Quad.BP_Quad_C"))
  (bind _output_get (Variables|Default|SetRootQuad _returnvalue))
  (Default|Initialise _output_get Knots (Utilities|Struct|MakeStruct_QuadData 0 0 Location Length KnotThreshold 0 "Root" "(R=0.000000,G=0.000000,B=0.000000,A=0.000000)" (Variables|Debug|GetDrawQuads?) (Variables|Debug|GetDrawCorners?) (Variables|Debug|GetDrawKnots?))))

(fn GetNearestKnot
  (params (SourceLocation :type Vector) (SourceRadius :type Float%20%28double-precision%29))
  (bind _overlappingquads (Default|GetOverlappingQuads (Variables|Default|GetRootQuad) SourceLocation SourceRadius))
  (for _array_element _overlappingquads
    (CallFunction|DebugDrawOverlappingQuads _array_element)
    (Utilities|Array|AppendArray (LocalVariables|Get_KnotsToSample) (Variables|/Game/Blueprint/PCG/BP_Quad.BP_Quad_C|GetKnots _array_element)))
  (for _array_element_2 (LocalVariables|Get_KnotsToSample)
    (if (< (Math|Vector|Distance2D(Vector) (Transformation|GetActorLocation _array_element_2) SourceLocation) (LocalVariables|Get_ClosestDistance))
      (LocalVariables|Set_ClosestDistance (Math|Vector|Distance2D(Vector) (Transformation|GetActorLocation _array_element_2) SourceLocation))
      (LocalVariables|Set_ClosestKnot _array_element_2)))
  (Debug|DebugDrawNearestKnot (LocalVariables|Get_ClosestKnot))
  (return (LocalVariables|Get_ClosestKnot)))

(fn DebugDrawNearestKnot
  (params (Knot :type Actor%20Object%20Reference))
  (bind _returnvalue (Transformation|GetActorLocation Knot))
  (Utilities|IsValid Knot
    (:Is%20Valid
      (if (Variables|Debug|GetDrawClosestKnot?)
        (Rendering|Debug|DrawDebugArrow (+ _returnvalue "0.000000,0.000000,1250.000000") (+ _returnvalue "0.000000,0.000000,500.000000") 5e+03 "(R=1.000000,G=1.000000,B=1.000000,A=1.000000)" 99.0 2e+01)))))

(fn DebugDrawOverlappingQuads
  (params (Quad :type BP%20Quad%20Object%20Reference))
  (bind _returnvalue (Default|GetLength Quad))
  (if (Variables|Debug|GetDrawOverlappingQuads?)
    (Rendering|Debug|DrawDebugBox (Default|GetLocation Quad) (Math|Vector|MakeVector _returnvalue _returnvalue 8e+02) "(R=0.000000,G=1.000000,B=1.000000,A=1.000000)" "0, 0, 0" 99.0 2e+01)))

(fn DebugDrawNearestKnottoDebugCube
  (bind _querydebugcube (Variables|Default|GetQueryDebugCube))
  (bind _cube (Variables|/Game/Blueprint/PCG/BP_QueryDebug.BP_QueryDebug_C|GetCube _querydebugcube))
  (bind _returnvalue (Transformation|GetWorldLocation _cube))
  (Utilities|IsValid (Variables|Default|GetQueryDebugCube)
    (:Is%20Valid
      (Class|KismetSystemLibrary|DrawDebugCylinder _returnvalue (+ _returnvalue "0.000000,0.000000,500.000000") 1.5e+03 12 "(R=1.000000,G=0.000000,B=1.000000,A=1.000000)" 99.0 1e+01 "World")
      (Knots|GetNearestKnot _returnvalue 1.5e+03))))

(fn BuildPathtoTarget
  (bind _array_element (Utilities|Array|ForEachLoopwithBreak (Variables|Default|GetKnots))
    (:LoopBody
      (switch Utilities|FlowControl|Switch|SwitchonEnum_Locations (Variables|/Game/Blueprint/PCG/BP_Knot.BP_Knot_C|GetLocation _array_element)
        (:NewEnumerator1
          (bind _output_get (LocalVariables|Set_CurrentKnot _array_element))
          (Utilities|Array|Add (LocalVariables|Get_ExcludedKnots) _output_get)
          ;[0.15 0.15 0.15 0.5] Get target knot
          (bind _array_element_2 (Utilities|Array|ForEachLoopwithBreak (Variables|Default|GetKnots) :!label _label)
            (:LoopBody
              (if (Utilities|Enum|Equal(Enum) (Variables|/Game/Blueprint/PCG/BP_Knot.BP_Knot_C|GetLocation _array_element_2) (Variables|/Game/Blueprint/PCG/BP_Knot.BP_Knot_C|GetTarget _array_element))
                (LocalVariables|Set_TargetKnot _array_element_2)
                (goto _label Break)))
            (:Completed
              (while (LocalVariables|Get_IsTargetReached?)
                (bind _closestknot (CallFunction|GetNearestKnottoTargetExluding (Transformation|GetActorLocation (LocalVariables|Get_CurrentKnot)) 2e+03 (LocalVariables|Get_ExcludedKnots) (LocalVariables|Get_TargetKnot)))
                (Paths|DrawPath (LocalVariables|Get_CurrentKnot) _closestknot)
                (bind _output_get_2 (LocalVariables|Set_CurrentKnot _closestknot))
                (if (== _output_get_2 (LocalVariables|Get_TargetKnot))
                  (LocalVariables|Set_IsTargetReached? false)
                  (else
                    (Utilities|Array|Add (LocalVariables|Get_ExcludedKnots) _output_get_2)))))))))))

(fn GetNearestKnotExluding
  (params (SourceLocation :type Vector) (SourceRadius :type Float%20%28double-precision%29) (ExcludedKnots :type Array%20of%20BP%20Knot%20Object%20References))
  ;[0.15 0.15 0.15 0.5] Get all knots in range
  (bind _overlappingquads (Default|GetOverlappingQuads (Variables|Default|GetRootQuad) SourceLocation SourceRadius))
  (for _array_element _overlappingquads
    (CallFunction|DebugDrawOverlappingQuads _array_element)
    (Utilities|Array|AppendArray (LocalVariables|Get_KnotsToSample) (Variables|/Game/Blueprint/PCG/BP_Quad.BP_Quad_C|GetKnots _array_element)))
  ;[0.15 0.15 0.15 0.5] Remove exluded knots
  (for _array_element_2 ExcludedKnots
    (Utilities|Array|RemoveItem (LocalVariables|Get_KnotsToSample) _array_element_2))
  ;[0.15 0.15 0.15 0.5] Get closest knot
  (for _array_element_3 (LocalVariables|Get_KnotsToSample)
    (if (< (Math|Vector|Distance2D(Vector) (Transformation|GetActorLocation _array_element_3) SourceLocation) (LocalVariables|Get_ClosestDistance))
      (LocalVariables|Set_ClosestDistance (Math|Vector|Distance2D(Vector) (Transformation|GetActorLocation _array_element_3) SourceLocation))
      (LocalVariables|Set_ClosestKnot _array_element_3)))
  (Debug|DebugDrawNearestKnot (LocalVariables|Get_ClosestKnot))
  (return (LocalVariables|Get_ClosestKnot)))

(fn GetNearestKnottoTargetExluding
  (params (SourceLocation :type Vector) (SourceRadius :type Float%20%28double-precision%29) (ExcludedKnots :type Array%20of%20BP%20Knot%20Object%20References) (TargetKnot :type BP%20Knot%20Object%20Reference))
  ;[0.15 0.15 0.15 0.5] Get all knots in range
  (bind _overlappingquads (Default|GetOverlappingQuads (Variables|Default|GetRootQuad) SourceLocation SourceRadius))
  (for _array_element _overlappingquads
    (CallFunction|DebugDrawOverlappingQuads _array_element)
    (Utilities|Array|AppendArray (LocalVariables|Get_KnotsToSample) (Variables|/Game/Blueprint/PCG/BP_Quad.BP_Quad_C|GetKnots _array_element)))
  ;[0.15 0.15 0.15 0.5] Remove exluded knots
  (for _array_element_2 ExcludedKnots
    (Utilities|Array|RemoveItem (LocalVariables|Get_KnotsToSample) _array_element_2))
  ;[0.15 0.15 0.15 0.5] Get closest knot
  (for _array_element_3 (LocalVariables|Get_KnotsToSample)
    (if (< (Math|Vector|Distance2D(Vector) (Transformation|GetActorLocation _array_element_3) (Transformation|GetActorLocation TargetKnot)) (LocalVariables|Get_ClosestDistance))
      (LocalVariables|Set_ClosestDistance (Math|Vector|Distance2D(Vector) (Transformation|GetActorLocation _array_element_3) (Transformation|GetActorLocation TargetKnot)))
      (LocalVariables|Set_ClosestKnot _array_element_3)))
  (Debug|DebugDrawNearestKnot (LocalVariables|Get_ClosestKnot))
  (return (LocalVariables|Get_ClosestKnot)))
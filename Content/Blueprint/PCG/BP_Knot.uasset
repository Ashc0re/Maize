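; BP_Knot is a PCG-folder grid node actor carrying a weight and G, H and F distances, apparently for A*-style pathfinding.
; Its Location enum drives setup: every type except one gets a red sphere in the construction script and a fixed weight from RegenerateWeight, while that one type gets a random weight.
; RepNotify handlers on the three distances refresh a debug text showing their values.
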(event EventBeginPlay)

(event Collision|EventActorBeginOverlap
  (params (OtherActor :type Actor%20Object%20Reference)))

(event EventTick
  (params (DeltaSeconds :type Float%20%28single-precision%29)))

(fn ConstructionScript
  (if (Utilities|Enum|NotEqual(Enum) (Variables|Default|GetLocation) "NewEnumerator4")
    (Rendering|Material|SetMaterial (Variables|Default|GetSphere) 0 "/Game/2D/Testing/M_SolidColour_Red.M_SolidColour_Red")))

(fn RegenerateWeight
  (if (Utilities|Enum|NotEqual(Enum) (Variables|Default|GetLocation) "NewEnumerator4")
    (Variables|Default|SetWeight 1.0)
    (else
      (Variables|Default|SetWeight (Math|Random|RandomFloatinRange 0.0 1.0)))))

(fn OnRepGDistance
  (CallFunction|SetDebugText))

(fn OnRepHDistance
  (CallFunction|SetDebugText))

(fn OnRepFDistance
  (CallFunction|SetDebugText))

(fn SetDebugText
  (Rendering|Components|TextRender|SetText (Variables|Default|GetDebugText) (Utilities|Text|FormatText "GDistance: {GDistance} 
HDistance: {HDistance} 
FDistance: {FDistance}" (Variables|Default|GetGDistance) (Variables|Default|GetHDistance) (Variables|Default|GetFDistance))))
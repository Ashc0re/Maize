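; BP_Quad is a quadtree node that spatially partitions Knot actors on the XY plane.
; When its Knot count exceeds the threshold, it adds four child quads to its owner at grid-snapped half size, recursively.
; Each child moves the Knots inside its bounds out of its parent.
; GetOverlappingQuads recursively collects leaf quads within a radius using a clamped closest-point test, with optional debug drawing of quads, corners and Knots.
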(fn Initialise
  (params (Knots :type Array%20of%20BP%20Knot%20Object%20References) (QuadData :type Struct%20Quad%20Data%20Structure))
  (Variables|Default|SetKnots Knots)
  (Variables|Default|SetQuadData QuadData)
  (Debug|DebugDrawQuad)
  (Knots|DelegateKnotsfromParent)
  ;[0.15 0.15 0.15 0.5] If there are too many knots in a quad, subdivide it.
  (if (> (Utilities|Array|Length (Variables|Default|GetKnots)) (QuadData|GetKnotThreshold))
    (Quad|Subdivide)))

(fn Subdivide
  (bind _returnvalue (QuadData|GetGeneration))
  (bind _self self)
  (bind _returnvalue_2 (+ 1 _returnvalue))
  (bind _quaddata (Variables|Default|GetQuadData _self))
  ;[0.15 0.15 0.15 0.5] Calculate subdivision length
  (LocalVariables|Set_SubdivisionLength (Math|Float|SnapToGrid(Float) (/ (QuadData|GetLength) 2.0) 5.0))
  (for _index (range 0 3)
    (bind _returnvalue_3 (Game|AddComponentbyClass (Components|GetOwner) "BP_Quad_C"))
    (LocalVariables|Set_CurrentSubdivision _returnvalue_3)
    (Quad|Initialise (LocalVariables|Get_CurrentSubdivision) 0 (Utilities|Struct|MakeStruct_QuadData _self 0 (+ (QuadData|GetLocation) (* (Utilities|Array|Get(acopy) (LocalVariables|Get_SubdivisionIndex) _index) (LocalVariables|Get_SubdivisionLength))) (LocalVariables|Get_SubdivisionLength) (.knotthreshold _quaddata) _returnvalue_2 (Utilities|String|Append "Quad " (Utilities|String|ToString(Integer) _returnvalue_2) "0" (Utilities|String|ToString(Integer) (+ _index 1))) (Math|Conversions|ToLinearColor(Vector) (* (Utilities|Array|Get(acopy) (LocalVariables|Get_SubdivisionIndex) _index) (LocalVariables|Get_SubdivisionLength))) (.deubg_drawquad? _quaddata) (.debug_drawcorners? _quaddata) (.debug_drawknots? _quaddata)))
    (Utilities|Array|Add (LocalVariables|Get_Subdivisions) (LocalVariables|Get_CurrentSubdivision))
    (Utilities|Struct|SetmembersinStruct_QuadData (Variables|Default|GetQuadData) (LocalVariables|Get_Subdivisions))))

(fn GetQuadCorner
  (params (X :type Float%20%28double-precision%29) (Y :type Float%20%28double-precision%29))
  (bind _returnvalue (QuadData|GetLength))
  (bind _returnvalue_2 (QuadData|GetLocation))
  (bind _returnvalue_3 (Math|Vector|MakeVector X Y 0.0))
  (bind _returnvalue_4 (* _returnvalue_3 _returnvalue))
  (bind _returnvalue_5 (+ _returnvalue_4 _returnvalue_2))
  (Debug|DebugDrawCorner _returnvalue_5)
  (return _returnvalue_5))

(fn GetAllQuadCorners
  (return (Quad|GetQuadCorner 1.0 1.0) (Quad|GetQuadCorner -1.0 -1.0)))

(fn IsKnotInsideBounds?
  (params (Knot :type Actor%20Object%20Reference) (TopRight :type Vector) (BottomLeft :type Vector))
  (bind _returnvalue (Transformation|GetActorLocation Knot))
  (bind (_x _y) (Math|Vector|BreakVector TopRight))
  (bind (_x_2 _y_2) (Math|Vector|BreakVector BottomLeft))
  (return (Math|Boolean|ANDBoolean (<= (.x _returnvalue) _x) (<= (.y _returnvalue) _y) (> (.y _returnvalue) _y_2) (> (.x _returnvalue) _x_2))))

(fn IsPointOverlappingQuad?
  (params (SourceLocation :type Vector) (SourceRadius :type Float%20%28double-precision%29))
  (bind (_topright _bottomleft) (Quad|GetAllQuadCorners))
  (bind (_x _y) (Math|Vector|BreakVector _bottomleft))
  (bind (_x_2 _y_2) (Math|Vector|BreakVector _topright))
  (return (>= SourceRadius (Math|Vector|Distance(Vector) SourceLocation (Math|Vector|MakeVector (Math|Float|Clamp(Float) (.x SourceLocation) _x _x_2) (Math|Float|Clamp(Float) (.y SourceLocation) _y _y_2) 0.0)))))

(fn DelegateKnotsfromParent
  (bind (_topright _bottomleft) (Quad|GetAllQuadCorners))
  (bind _returnvalue (QuadData|GetParentQuad))
  ;[0.15 0.15 0.15 0.5] Skips root
  (Utilities|IsValid _returnvalue
    (:Is%20Valid
      (for _array_element (Variables|BP_Quad_C|GetKnots _returnvalue)
        (bind _output_get (LocalVariables|SetCurrentKnot _array_element))
        (if (Knots|IsKnotInsideBounds? _output_get _topright _bottomleft)
          (Utilities|Array|Add (Variables|Default|GetKnots) (LocalVariables|GetCurrentKnot))
          (Debug|DebugDrawKnot (LocalVariables|GetCurrentKnot))))
      (for _array_element_2 (Variables|Default|GetKnots)
        (Utilities|Array|RemoveItem (Variables|BP_Quad_C|GetKnots (QuadData|GetParentQuad)) _array_element_2)))))

(fn GetOverlappingQuads
  (params (SourceLocation :type Vector) (SourceRadius :type Float%20%28double-precision%29))
  (if (Knots|IsPointOverlappingQuad? SourceLocation SourceRadius)
    (if (> (Utilities|Array|Length (QuadData|GetSubdivisions)) 0)
      (for _array_element (QuadData|GetSubdivisions)
        (bind _overlappingquads (Quad|GetOverlappingQuads _array_element SourceLocation SourceRadius))
        (Utilities|Array|AppendArray (LocalVariables|Get_OverlappingQuads) _overlappingquads))
      (else
        (Utilities|Array|Add (LocalVariables|Get_OverlappingQuads) self)))
    (return (LocalVariables|Get_OverlappingQuads))))

(fn DebugDrawQuad
  (bind _returnvalue (QuadData|GetLength))
  (if (QuadData|GetDrawDebugQuad?)
    (Rendering|Debug|DrawDebugBox (QuadData|GetLocation) (Math|Vector|MakeVector _returnvalue _returnvalue 5e+02) (QuadData|GetDebugColor) "0, 0, 0" 99.0 5.0)))

(fn DebugDrawCorner
  (params (Center :type Vector))
  (if (QuadData|GetDrawDebugCorners?)
    (Rendering|Debug|DrawDebugCapsule Center 5.2e+02 2e+01 "0, 0, 0" (QuadData|GetDebugColor) 99.0 5.0))
  (return))

(fn DebugDrawKnot
  (params (Knot :type Actor%20Object%20Reference))
  (bind _returnvalue (Transformation|GetActorLocation Knot))
  (if (QuadData|GetDrawDebugKnots?)
    (Class|KismetSystemLibrary|DrawDebugCylinder _returnvalue (+ _returnvalue "0.000000,0.000000,400.000000") 1e+02 12 (QuadData|GetDebugColor) 99.0 2e+01 "World")))

(fn GetParentQuad
  (return (.parentquad (Variables|Default|GetQuadData))))

(fn GetSubdivisions
  (return (.subdivisions (Variables|Default|GetQuadData))))

(fn GetLocation
  (return (.location (Variables|Default|GetQuadData))))

(fn GetLength
  (return (.length (Variables|Default|GetQuadData))))

(fn GetKnotThreshold
  (return (.knotthreshold (Variables|Default|GetQuadData))))

(fn GetGeneration
  (return (.generation (Variables|Default|GetQuadData))))

(fn GetDebugName
  (return (.debug_name (Variables|Default|GetQuadData))))

(fn GetDebugColor
  (return (.debug_color (Variables|Default|GetQuadData))))

(fn GetDrawDebugQuad?
  (return (.deubg_drawquad? (Variables|Default|GetQuadData))))

(fn GetDrawDebugCorners?
  (return (.debug_drawcorners? (Variables|Default|GetQuadData))))

(fn GetDrawDebugKnots?
  (return (.debug_drawknots? (Variables|Default|GetQuadData))))
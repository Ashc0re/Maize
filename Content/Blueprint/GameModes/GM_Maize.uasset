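; GM_Maize is a game mode that starts a new session and places the player in the level.
; On BeginPlay it writes a "New Game Session" banner to the log, then gathers all PlayerStart actors.
; It manually spawns the default pawn class at the first one found and has player controller 0 possess it, breaking out of the loop immediately.
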(event EventBeginPlay
  (Utilities|String|LogString (Utilities|String|Append "///////////////////////" "New Game Session" "//////////////////////"))
  (bind _outactors (Actor|GetAllActorsOfClass "/Script/Engine.PlayerStart"))
  (bind _array_element (Utilities|Array|ForEachLoopwithBreak _outactors :!label _label)
    (:LoopBody
      (bind _returnvalue (Game|SpawnActorfromClass (Variables|/Script/Engine.GameModeBase|GetDefaultPawnClass (Game|GetGameMode)) (Transformation|GetActorTransform _array_element) "Undefined" "MultiplyWithRoot" (Game|GetPlayerController 0) 0))
      (Pawn|Possess (Game|GetPlayerController 0) _returnvalue)
      (goto _label Break))))

(fn ConstructionScript)
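; Stationary scarecrow Blueprint that periodically turns its head bone on a poseable mesh.
; On BeginPlay it starts a looping HeadTurn timeline, with HeadTurnRate setting the interval between Head Turn events.
; Each event calculates a head rotation and applies it in world space only when the look-at validity check accepts the yaw.
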(event EventBeginPlay
  (|CallParentFunction)
  (CallFunction|SetUpHeadTurn)
  (Timeline|HeadTurn Play
    (:HeadTurn
      (bind (_yaw _rotation) (CallFunction|CalculateHeadRotation))
      (bind _isvalid (CallFunction|CheckLookatValidity _yaw))
      (if _isvalid
        (Components|PoseableMesh|SetBoneRotationbyName (Variables|Default|GetPoseableMesh) "head" _rotation "WorldSpace")))))

(fn ConstructionScript
  (|CallParentFunction))

(fn SetUpHeadTurn
  (Components|Timeline|SetPlayRate (Variables|Default|GetHeadTurn) (/ 1.0 (Variables|Default|GetHeadTurnRate)))
  (Components|Timeline|SetLooping (Variables|Default|GetHeadTurn) true)
  (return))
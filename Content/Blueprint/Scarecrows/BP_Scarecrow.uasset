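; Scarecrow actor with a poseable mesh whose head bone gets a random world-space rotation at BeginPlay, if the player character is valid.
; Helper functions compute a jittered, axis-offset look-at rotation from head to player capsule and check LookAtRange overlap plus an angle window.
; Neither look-at helper is called within this Blueprint, so the head does not track the player here.
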(event EventBeginPlay
  (Utilities|IsValid (Game|GetPlayerCharacter 0)
    (:Is%20Valid
      (CallFunction|SetRandomHeadRotation))))

(fn ConstructionScript)

(fn SetRandomHeadRotation
  (Components|PoseableMesh|SetBoneRotationbyName (Variables|Default|GetPoseableMesh) "head" (Math|Rotator|MakeRotator (Math|Random|RandomFloatinRange -3e+01 5e+01) (Math|Random|RandomFloatinRange 7e+01 1.1e+02) (Math|Random|RandomFloatinRange -1e+01 4e+01)) "WorldSpace"))

(fn CheckLookatValidity
  (params (Value :type Float%20%28double-precision%29))
  (return (and (Collision|IsOverlappingActor (Variables|Default|GetLookAtRange) (Game|GetPlayerCharacter 0) :!class /Script/Engine.PrimitiveComponent) (Math|Float|InRange(Float) Value 2e+01 1.6e+02))))

(fn CalculateHeadRotation
  (bind _returnvalue (Math|Random|RandomFloatinRange 85.0 95.0))
  (bind _returnvalue_2 (Game|GetPlayerCharacter 0))
  (bind _poseablemesh (Variables|Default|GetPoseableMesh))
  (bind _returnvalue_3 (Transformation|GetBoneTransform _poseablemesh "head" "RTS_World"))
  (bind _capsulecomponent (Variables|/Script/Engine.Character|GetCapsuleComponent _returnvalue_2))
  (bind _returnvalue_4 (Transformation|GetWorldLocation _capsulecomponent))
  (bind _returnvalue_5 (Math|Rotator|FindLookatRotation (.location _returnvalue_3) _returnvalue_4))
  (bind (_roll _pitch _yaw) (Math|Rotator|BreakRotator _returnvalue_5))
  (Utilities|IsValid _returnvalue_2
    (:Is%20Valid
      (return _yaw (Math|Rotator|MakeRotator (+ _roll _returnvalue) (+ _pitch _returnvalue) _yaw)))))
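; Base player character with movement, crouch, look, timed hold-to-interact and a stackable slot inventory.
; A sphere trace selects BP_Interactable targets, then timelines re-trace while filling InteractProgress and notify the target actor when finished.
; POI mode disables movement, blends to the POI's camera with clamped look and allows component-level interaction until right-click exits.
; RepNotifies on InteractProgress and Inventory refresh the interact bar and inventory widgets through BP_PlayerController's UI.
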(event Custom|Event_InteractWithComponent
  (params (InteractTime :type Float%20%28double-precision%29) (InteractActor :type BP%20Interactable%20Object%20Reference) (InteractComponent :type Primitive%20Component%20Object%20Reference))
  ;[0.15 0.15 0.15 0.5] Interaction Logic and Function Calling
  (Utilities|IsValid InteractActor
    (:Is%20Valid
      (Components|Timeline|SetPlayRate (Variables|Default|GetTL_InteractWithComponent) (/ 1.0 InteractTime))
      (bind _progress (Timeline|TL_InteractWithComponent PlayFromStart)
        (:Update
          (bind _outhit (Interaction|InteractTrace))
          (if (== (.HitComponent (Collision|BreakHitResult _outhit)) InteractComponent)
            (Variables|Default|SetInteractProgress _progress)
            (else
              (CallFunction|EventEndComponentInteraction)
              (Development|PrintString "Hello"))))
        (:Finished
          (Default|InteractedwithComponent InteractActor InteractComponent self))))))

(event Custom|Event_EndComponentInteraction
  ;[0.15 0.15 0.15 0.5] Interaction Logic and Function Calling
  (Variables|Default|SetInteractProgress 0.0)
  (bind _progress (Timeline|TL_InteractWithComponent Stop)
    (:Update
      (bind _outhit (Interaction|InteractTrace))
      (if (== (.HitComponent (Collision|BreakHitResult _outhit)) (stale Custom|Event_InteractWithComponent InteractComponent))
        (Variables|Default|SetInteractProgress _progress)
        (else
          (CallFunction|EventEndComponentInteraction)
          (Development|PrintString "Hello"))))
    (:Finished
      (Default|InteractedwithComponent (stale Custom|Event_InteractWithComponent InteractActor) (stale Custom|Event_InteractWithComponent InteractComponent) self))))

(event Custom|Event_EndActorInteraction
  ;[0.15 0.15 0.15 0.5] Interaction Logic and Function Calling
  (Variables|Default|SetInteractProgress 0.0)
  (bind _progress (Timeline|TL_InteractWithActor Stop)
    (:Update
      (bind _outhit (Interaction|InteractTrace))
      (if (== (.HitActor (Collision|BreakHitResult _outhit)) (stale Custom|Event_InteractWithActor InteractActor))
        (Variables|Default|SetInteractProgress _progress)
        (else
          (CallFunction|EventEndActorInteraction))))
    (:Finished
      (Default|InteractedwithActor (stale Custom|Event_InteractWithActor InteractActor) self))))

(event Custom|Event_EnterPOI
  (params (POIActor :type BP%20POI%20Object%20Reference))
  ;[0.15 0.15 0.15 0.5] POIs
  ;;[0.15 0.15 0.15 0.5] Entering POIs
  (Utilities|IsValid POIActor
    (:Is%20Valid
      (bind _output_get (Variables|Default|SetCurrentPOIActor POIActor))
      (Variables|Default|SetInPOIMode true)
      (Pawn|Components|CharacterMovement|DisableMovement (Variables|Character|GetCharacterMovement))
      (Game|Player|SetViewTargetwithBlend (Game|GetPlayerController 0) _output_get 0.5 "VTBlend_Linear" 0.0 false))))

(event Custom|Event_LeavePOI
  ;[0.15 0.15 0.15 0.5] POIs
  ;;[0.15 0.15 0.15 0.5] Leaving POIs
  (if (Variables|Default|GetInPOIMode)
    (Pawn|Components|CharacterMovement|SetMovementMode (Variables|Character|GetCharacterMovement) "MOVE_Walking" 0)
    (Game|Player|SetViewTargetwithBlend (Game|GetPlayerController 0) self 0.5 "VTBlend_Linear" 0.0 false)
    (Variables|Default|SetInPOIMode false)
    (Variables|/Game/Blueprint/Interactables/BP_Interactable.BP_Interactable_C|SetCurrentlyInteractable (Variables|Default|GetCurrentPOIActor) true)
    (Variables|Default|SetCurrentPOIActor 0)))

(event Custom|Event_InteractWithActor
  (params (InteractTime :type Float%20%28double-precision%29) (InteractActor :type BP%20Interactable%20Object%20Reference))
  ;[0.15 0.15 0.15 0.5] Interaction Logic and Function Calling
  (Utilities|IsValid InteractActor
    (:Is%20Valid
      (Components|Timeline|SetPlayRate (Variables|Default|GetTL_InteractWithActor) (/ 1.0 InteractTime))
      (bind _progress (Timeline|TL_InteractWithActor PlayFromStart)
        (:Update
          (bind _outhit (Interaction|InteractTrace))
          (if (== (.HitActor (Collision|BreakHitResult _outhit)) InteractActor)
            (Variables|Default|SetInteractProgress _progress)
            (else
              (CallFunction|EventEndActorInteraction))))
        (:Finished
          (Default|InteractedwithActor InteractActor self))))))

(event Input|EnhancedActionEvents|EnhancedInputActionIA_Crouch
  (params (ActionValue :type Boolean) (ElapsedSeconds :type Float%20%28double-precision%29) (TriggeredSeconds :type Float%20%28double-precision%29) (InputAction :type Input%20Action%20Object%20Reference :default "/Game/Blueprint/Player/Controls/IA_Crouch.IA_Crouch"))
  ;[0.15 0.15 0.15 0.5] Controls
  ;;[0.15 0.15 0.15 0.5] Movement
  ;;;[0.15 0.15 0.15 0.5] Crouching
  (:Started
    (Character|Crouch))
  (:Canceled
    (Character|UnCrouch)))

(event Input|EnhancedActionEvents|EnhancedInputActionIA_Move
  (params (ActionValue :type Vector%202D%20Structure) (ElapsedSeconds :type Float%20%28double-precision%29) (TriggeredSeconds :type Float%20%28double-precision%29) (InputAction :type Input%20Action%20Object%20Reference :default "/Game/Blueprint/Player/Controls/IA_Move.IA_Move"))
  ;[0.15 0.15 0.15 0.5] Controls
  ;;[0.15 0.15 0.15 0.5] Movement
  ;;;[0.15 0.15 0.15 0.5] Walking
  (Pawn|Input|AddMovementInput (Math|Vector|GetForwardVector (Variables|Collision|GetCapsuleComponent)) (.x ActionValue) false)
  (Pawn|Input|AddMovementInput (Math|Vector|GetRightVector (Variables|Collision|GetCapsuleComponent)) (.y ActionValue) false))

(event Input|EnhancedActionEvents|EnhancedInputActionIA_Look
  (params (ActionValue :type Vector%202D%20Structure) (ElapsedSeconds :type Float%20%28double-precision%29) (TriggeredSeconds :type Float%20%28double-precision%29) (InputAction :type Input%20Action%20Object%20Reference :default "/Game/Blueprint/Player/Controls/IA_Look.IA_Look"))
  ;[0.15 0.15 0.15 0.5] Controls
  ;;[0.15 0.15 0.15 0.5] Movement
  ;;;[0.15 0.15 0.15 0.5] Camera
  (Movement|CameraMovement (.x ActionValue) (.y ActionValue)))

(event Input|EnhancedActionEvents|EnhancedInputActionIA_Inventory
  (params (ActionValue :type Boolean) (ElapsedSeconds :type Float%20%28double-precision%29) (TriggeredSeconds :type Float%20%28double-precision%29) (InputAction :type Input%20Action%20Object%20Reference :default "/Game/Blueprint/Player/Controls/IA_Inventory.IA_Inventory"))
  ;[0.15 0.15 0.15 0.5] Controls
  ;;[0.15 0.15 0.15 0.5] UI
  ;;;[0.15 0.15 0.15 0.5] Inventory
  (:Triggered
    (bind _uielement (UI|GetUIComponent "NewEnumerator1"))
    (Widget|SetVisibility _uielement "HitTestInvisible")
    (UI|UpdateInventory))
  (:Canceled
    (bind _uielement_2 (UI|GetUIComponent "NewEnumerator1" :!label _label))
    (Widget|SetVisibility _uielement_2 "Hidden"))
  (:Completed
    (goto _label)))

(event Input|EnhancedActionEvents|EnhancedInputActionIA_Interact
  (params (ActionValue :type Boolean) (ElapsedSeconds :type Float%20%28double-precision%29) (TriggeredSeconds :type Float%20%28double-precision%29) (InputAction :type Input%20Action%20Object%20Reference :default "/Game/Blueprint/Player/Controls/IA_Interact.IA_Interact"))
  ;[0.15 0.15 0.15 0.5] Controls
  ;;[0.15 0.15 0.15 0.5] Interaction
  ;;;[0.15 0.15 0.15 0.5] Interact Input and Sphere Trace
  (:Started
    (bind _outhit (Interaction|InteractTrace))
    (Interaction|SelectInteractBehaviour (.HitActor (Collision|BreakHitResult _outhit)) (.HitComponent (Collision|BreakHitResult _outhit))))
  (:Canceled
    (CallFunction|EventEndActorInteraction :!label _label)
    (CallFunction|EventEndComponentInteraction))
  (:Completed
    (goto _label)))

(event Input|MouseEvents|RightMouseButton
  (params (Key :type Key%20Structure :default "None"))
  ;[0.15 0.15 0.15 0.5] Controls
  ;;[0.15 0.15 0.15 0.5] Interaction
  ;;;[0.15 0.15 0.15 0.5] Other
  (:Released
    (CallFunction|EventLeavePOI)))

(fn ConstructionScript)

(fn InventoryAddItem
  (params (ItemToAdd :type BP%20Item%20Base%20Class%20Reference) (ItemQuantity :type Integer))
  (LocalVariables|Set_ItemToAdd ItemToAdd)
  (LocalVariables|Set_ItemQuantity ItemQuantity)
  (for (_array_element _array_index) (Variables|Default|GetInventory)
    ;[0.15 0.15 0.15 0.5] Override Item Slot if Item is already present and the stack isn't full
    (LocalVariables|Set_InventoryIndex _array_index)
    (if (and (== (LocalVariables|Get_ItemToAdd) (.Item_Class (Utilities|Struct|BreakStruct_Item _array_element))) (< (.Item_Quantity (Utilities|Struct|BreakStruct_Item _array_element)) (.Item_MaxStackSize (Utilities|Struct|BreakStruct_Item _array_element))))
      (Utilities|Array|SetArrayElem (Variables|Default|GetInventory) (LocalVariables|Get_InventoryIndex) (Utilities|Struct|MakeStruct_Item (LocalVariables|Get_ItemToAdd) (+ (.Item_Quantity (Utilities|Struct|BreakStruct_Item _array_element)) (LocalVariables|Get_ItemQuantity)) (.Item_MaxStackSize (Utilities|Struct|BreakStruct_Item _array_element))))
      (return true)))
  ;[0.15 0.15 0.15 0.5] If no such slot was found, use the first empty slot
  (bind (_array_element_2 _array_index_2) (Utilities|Array|ForEachLoopwithBreak (Variables|Default|GetInventory))
    (:LoopBody
      (if (== (.Item_Class (Utilities|Struct|BreakStruct_Item _array_element_2)) "/Game/Blueprint/Interactables/PickUps/Items/_BP_Item_Empty._BP_Item_Empty_C")
        (Utilities|Array|SetArrayElem (Variables|Default|GetInventory) _array_index_2 (Utilities|Struct|MakeStruct_Item (LocalVariables|Get_ItemToAdd) (.Amount (Utilities|GetClassDefaults (LocalVariables|Get_ItemToAdd))) (.StackSize (Utilities|GetClassDefaults (LocalVariables|Get_ItemToAdd)))))
        (return true)))
    (:Completed
      (return false))))

(fn InteractTrace
  (if (Variables|Default|GetInPOIMode)
    (LocalVariables|Set_InteractCam (Variables|/Game/Blueprint/Interactables/POIs/BP_POI.BP_POI_C|GetCamera_Inspect (Variables|Default|GetCurrentPOIActor)))
    (LocalVariables|Set_InteractRadius 1.0)
    (else
      (LocalVariables|Set_InteractCam (Variables|Default|GetCamera_Gameplay))
      (LocalVariables|Set_InteractRadius 5.0)))
  (bind _outhit (Collision|SphereTraceForObjects (Transformation|GetWorldLocation (LocalVariables|Get_InteractCam)) (+ (Transformation|GetWorldLocation (LocalVariables|Get_InteractCam)) (* (Math|Vector|GetForwardVector (LocalVariables|Get_InteractCam)) 5e+02)) (LocalVariables|Get_InteractRadius) (Variables|Default|GetInteractObjects) false (Variables|Default|GetInteractActorsToIgnore) "ForDuration"))
  (return _outhit))

(fn OnRepInteractProgress
  (bind _uielement (UI|GetUIComponent "NewEnumerator2"))
  (bind _aswbp_interact_bar (Utilities|Casting|CastToWBP_InteractBar _uielement))
  (Default|EventUpdateInteractProgress _aswbp_interact_bar (Variables|Default|GetInteractProgress)))

(fn OnRepInventory
  (UI|UpdateInventory))

(fn UpdateInventory
  (bind _uielement (UI|GetUIComponent "NewEnumerator1"))
  (bind _aswbp_inventory (Utilities|Casting|CastToWBP_Inventory _uielement))
  (for _index (range 0 (- (Utilities|Array|Length (Variables|Default|GetInventory)) 1))
    (LocalVariables|SetCurrentIndex _index)
    (bind _aswbp_item (Utilities|Casting|CastToWBP_Item (Class|PanelWidget|GetChildat (Variables|/Game/Blueprint/UI/UIElements/WBP_Inventory.WBP_Inventory_C|GetGrid _aswbp_inventory) _index)))
    (Default|EventUpdateWidget _aswbp_item (.Item_Quantity (Utilities|Struct|BreakStruct_Item (Utilities|Array|Get(acopy) (Variables|Default|GetInventory) (LocalVariables|GetCurrentIndex)))) (.Image (Utilities|GetClassDefaults (.Item_Class (Utilities|Struct|BreakStruct_Item (Utilities|Array|Get(acopy) (Variables|Default|GetInventory) (LocalVariables|GetCurrentIndex)))))))))

(fn GetUIComponent
  (params (ElementToGet :type Enum_UIElements%20Enum :default "NewEnumerator0"))
  (bind _asbp_player_controller (Utilities|Casting|CastToBP_PlayerController (Game|GetPlayerController 0)))
  (LocalVariables|Set_PlayerController _asbp_player_controller)
  (switch Utilities|FlowControl|Switch|SwitchonEnum_UIElements ElementToGet
    (:NewEnumerator0
      (LocalVariables|Set_ElementToReturn (Variables|/Game/Blueprint/Player/BP_PlayerController.BP_PlayerController_C|GetUI (LocalVariables|Get_PlayerController))))
    (:NewEnumerator1
      (LocalVariables|Set_ElementToReturn (Variables|/Game/Blueprint/UI/WBP_UI.WBP_UI_C|GetWBP_Inventory (Variables|/Game/Blueprint/Player/BP_PlayerController.BP_PlayerController_C|GetUI (LocalVariables|Get_PlayerController)))))
    (:NewEnumerator2
      (LocalVariables|Set_ElementToReturn (Variables|/Game/Blueprint/UI/WBP_UI.WBP_UI_C|GetWBP_InteractBar (Variables|/Game/Blueprint/Player/BP_PlayerController.BP_PlayerController_C|GetUI (LocalVariables|Get_PlayerController))))))
  (return (LocalVariables|Get_ElementToReturn)))

(fn CameraMovement
  (params (X%20Axis :type Float%20%28single-precision%29) (Y%20Axis :type Float%20%28single-precision%29))
  (bind _currentpoiactor (Variables|Default|GetCurrentPOIActor))
  (bind _camera_inspect (Variables|/Game/Blueprint/Interactables/POIs/BP_POI.BP_POI_C|GetCamera_Inspect _currentpoiactor))
  (bind _relativerotation (Variables|/Script/Engine.SceneComponent|GetRelativeRotation _camera_inspect))
  (LocalVariables|Set_XAxis X%20Axis)
  (LocalVariables|Set_YAxis Y%20Axis)
  (if (Variables|Default|GetInPOIMode)
    ;[0.15 0.15 0.15 0.5] POI Camera
    (Utilities|IsValid _currentpoiactor
      (:Is%20Valid
        (Transformation|SetRelativeRotation _camera_inspect (Math|Rotator|MakeRotator 0.0 (Math|Float|Clamp(Float) (+ (.pitch _relativerotation) (* (LocalVariables|Get_YAxis) -1.0)) -25.0 25.0) (Math|Float|Clamp(Float) (+ (.yaw _relativerotation) (LocalVariables|Get_XAxis)) -2e+01 2e+01)) false false)))
    (else
      ;[0.15 0.15 0.15 0.5] Gameplay Camera
      (Pawn|Input|AddControllerPitchInput (LocalVariables|Get_YAxis))
      (Pawn|Input|AddControllerYawInput (LocalVariables|Get_XAxis)))))

(fn SelectInteractBehaviour
  (params (HitActor :type Object%20Object%20Reference) (HitComponent :type Primitive%20Component%20Object%20Reference))
  (Utilities|FlowControl|Sequence
    (:then_0
      (Utilities|IsValid HitComponent
        (:Is%20Valid
          (LocalVariables|Set_HitComponent HitComponent))))
    (:then_1
      (bind _asbp_interactable (Utilities|Casting|CastToBP_Interactable HitActor))
      (LocalVariables|Set_HitActor _asbp_interactable)
      (if (Variables|/Game/Blueprint/Interactables/BP_Interactable.BP_Interactable_C|GetCurrentlyInteractable (LocalVariables|Get_HitActor))
        (switch Utilities|FlowControl|Switch|SwitchonEnum_InteractableType (Variables|/Game/Blueprint/Interactables/BP_Interactable.BP_Interactable_C|GetInteractableType (LocalVariables|Get_HitActor))
          (:NewEnumerator0
            (CallFunction|EventInteractwithActor (Variables|/Game/Blueprint/Interactables/BP_Interactable.BP_Interactable_C|GetInteractTime (LocalVariables|Get_HitActor))))
          (:NewEnumerator1
            (bind _asbp_poi (Utilities|Casting|CastToBP_POI (LocalVariables|Get_HitActor)))
            (if (Variables|/Game/Blueprint/Interactables/POIs/BP_POI.BP_POI_C|GetDirectlyInteractable _asbp_poi)
              (if (Components|ComponentHasTag (LocalVariables|Get_HitComponent) "Interactable")
                (CallFunction|EventInteractwithComponent (Variables|/Game/Blueprint/Interactables/BP_Interactable.BP_Interactable_C|GetInteractTime (LocalVariables|Get_HitActor)) (LocalVariables|Get_HitActor) (LocalVariables|Get_HitComponent)))
              (elif (not (Variables|Default|GetInPOIMode))
                (Variables|/Game/Blueprint/Interactables/BP_Interactable.BP_Interactable_C|SetCurrentlyInteractable (LocalVariables|Get_HitActor) false)
                (CallFunction|EventEnterPOI _asbp_poi)))))
        (elif (Variables|Default|GetInPOIMode)
          (Development|PrintString (Utilities|String|ToString(Float) (Variables|/Game/Blueprint/Interactables/BP_Interactable.BP_Interactable_C|GetInteractTime (LocalVariables|Get_HitActor))))
          (CallFunction|EventInteractwithComponent (Variables|/Game/Blueprint/Interactables/BP_Interactable.BP_Interactable_C|GetInteractTime (LocalVariables|Get_HitActor)) (LocalVariables|Get_HitActor) (LocalVariables|Get_HitComponent)))))))

(fn InventoryRemoveItem
  (params (ItemToRemove :type BP%20Item%20Base%20Class%20Reference) (QuantityToRemove :type Integer))
  (LocalVariables|Set_QuantityToRemove QuantityToRemove)
  (for (_array_element _array_index) (Variables|Default|GetInventory)
    (LocalVariables|Set_ItemIndex _array_index)
    (LocalVariables|Set_QuantityPresent (.Item_Quantity (Utilities|Struct|BreakStruct_Item _array_element)))
    (if (== (.Item_Class (Utilities|Struct|BreakStruct_Item _array_element)) ItemToRemove)
      (if (== (LocalVariables|Get_QuantityPresent) (LocalVariables|Get_QuantityToRemove))
        (Utilities|Array|SetArrayElem (Variables|Default|GetInventory) (LocalVariables|Get_ItemIndex) (Utilities|Struct|MakeStruct_Item "/Game/Blueprint/Interactables/PickUps/Items/_BP_Item_Empty._BP_Item_Empty_C" 0 0))
        (UI|UpdateInventory)
        (elif (> (LocalVariables|Get_QuantityPresent) (LocalVariables|Get_QuantityToRemove))
          (Utilities|Array|SetArrayElem (Variables|Default|GetInventory) (LocalVariables|Get_ItemIndex) (Utilities|Struct|MakeStruct_Item (.Item_Class (Utilities|Struct|BreakStruct_Item (Utilities|Array|Get(acopy) (Variables|Default|GetInventory) (LocalVariables|Get_ItemIndex)))) (- (.Item_Quantity (Utilities|Struct|BreakStruct_Item (Utilities|Array|Get(acopy) (Variables|Default|GetInventory) (LocalVariables|Get_ItemIndex)))) (LocalVariables|Get_QuantityToRemove)) (.Item_MaxStackSize (Utilities|Struct|BreakStruct_Item (Utilities|Array|Get(acopy) (Variables|Default|GetInventory) (LocalVariables|Get_ItemIndex))))))
          (UI|UpdateInventory))))))

(fn CarriesItem
  (params (ItemsToCheck :type Array%20of%20BP%20Item%20Base%20Class%20References))
  (bind _array_element (Utilities|Array|ForEachLoopwithBreak ItemsToCheck)
    (:LoopBody
      (bind _array_element_2 (Utilities|Array|ForEachLoopwithBreak (Variables|Default|GetInventory) :!label _label)
        (:LoopBody
          (if (== _array_element (.Item_Class (Utilities|Struct|BreakStruct_Item _array_element_2)))
            (Utilities|Array|Add (LocalVariables|Get_ItemsPresent) true)
            (goto _label Break)))))
    (:Completed
      (if (== (Utilities|Array|Length ItemsToCheck) (Utilities|Array|Length (LocalVariables|Get_ItemsPresent)))
        (return true)
        (else
          (return false))))))